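; BP_TBSGrid is a TBS grid actor that displays a tiled grid through a material on its GridComponent.
; The construction script creates a dynamic instance of M_GridMat and applies it to the component's first material slot.
; On BeginPlay, GridWidth and GridHeight set the material's U and V tiling, with debug prints of both, and the opacity multiplier is set to full.
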(event `self.ReceiveBeginPlay`
  (`MaterialInstanceDynamic.SetScalarParameterValue` (`self.DynamicGridMaterial`) "UTiling" (`KismetMathLibrary.Conv_IntToDouble` (`self.GridWidth`)))
  (`KismetSystemLibrary.PrintString` (`KismetStringLibrary.Conv_IntToString` (`self.GridWidth`)))
  (`MaterialInstanceDynamic.SetScalarParameterValue` (`self.DynamicGridMaterial`) "VTiling" (`KismetMathLibrary.Conv_IntToDouble` (`self.GridHeight`)))
  (`KismetSystemLibrary.PrintString` (`KismetStringLibrary.Conv_IntToString` (`self.GridHeight`)))
  (`MaterialInstanceDynamic.SetScalarParameterValue` (`self.DynamicGridMaterial`) "OpacityMultiplier" 1.0))

(fn `UserConstructionScript`
  (bind _returnvalue (`KismetMaterialLibrary.CreateDynamicMaterialInstance` "/Game/Materials/M_GridMat.M_GridMat"))
  (bind _output_get (set `self.DynamicGridMaterial` _returnvalue))
  (`PrimitiveComponent.SetMaterial` (`self.GridComponent`) 0 _output_get))